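; Player controller for the main game level that handles local UI, chat and player input.
; It creates chat and leaderboard widgets for the local player, and relays submitted chat to every controller in the GameState's PlayerArray.
; Input drives start/tick/end fire calls with camera shake, jumping and item drops.
; Map and Enter input, posture changes, item pickups and bullet-count updates are forwarded to the HUD.
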(event `Key|Tab`
  (params (Key :type "Key Structure"))
  (bind _ui_ref (`self.UI_Ref`))
  (:`Pressed`
    (`/Game/BluePrint/PartDevLevel/UI/LeaderBoard/WB_LeaderBoard.ShowList` _ui_ref true))
  (:`Released`
    (`/Game/BluePrint/PartDevLevel/UI/LeaderBoard/WB_LeaderBoard.ShowList` _ui_ref false)))

(event `self.ReceiveBeginPlay`
  ;[1 1 1] 플레이어에게 채팅창 좌측하단에 생성(UI)
  (`self.SetUpWeaponUI`)
  (if (`self.IsLocalController`)
    (bind _returnvalue (`|CreateWidget` "/Game/BluePrint/PartDevLevel/UI/chat/WB_ChatPanel.WB_ChatPanel_C" self))
    (bind _output_get (set `self.WB_Chat Panel ` _returnvalue))
    (`UserWidget.AddToViewport` _output_get 0)))

(event `self.ReceiveTick`
  (params (DeltaSeconds :type "Float (single-precision)")))

(event `Key|Enter`
  (params (Key :type "Key Structure"))
  ;[1 1 1] 채팅창(UI)
  ;;[1 1 1] 엔터시 채팅창으로 키보드 포커스 이동
  (:`Pressed`
    (bind _wb_chat_panel_ (`self.WB_Chat Panel `)
      (:`then`
        (`Widget.SetKeyboardFocus` (`/Game/BluePrint/PartDevLevel/UI/chat/WB_ChatPanel.ChatInputBox` _wb_chat_panel_)))
      (:`else`))))

(event `SR_SubmiChat`
  (params (PlayerName :type Text) (ChatMassage :type Text))
  ;[1 1 1] 채팅창(UI)
  (for _array_element (`GameStateBase.PlayerArray` (`GameplayStatics.GetGameState`))
    (bind _asbp_character_controller (cast `/Game/BluePrint/MainGameLevel/Character/BP_CharacterController` (`PlayerState.GetPlayerController` _array_element)))
    (`self.OC_UpdateChat` _asbp_character_controller PlayerName ChatMassage)))

(event `OC_UpdateChat`
  (params (`Player Name` :type Text) (`Chat Massage` :type Text))
  ;[1 1 1] 채팅창(UI)
  (bind _wb_chat_panel_ (`self.WB_Chat Panel `)
    (:`then`
      (`/Game/BluePrint/PartDevLevel/UI/chat/WB_ChatPanel.Update_Chat` _wb_chat_panel_ `Player Name` `Chat Massage`))
    (:`else`)))

(event `EnhancedInput|/Game/Resources/TestLevel/Input/IA_Fire`
  (params (ActionValue :type Boolean) (ElapsedSeconds :type "Float (double-precision)") (TriggeredSeconds :type "Float (double-precision)") (InputAction :type "InputAction Object Reference" :default "/Game/Resources/TestLevel/Input/IA_Fire.IA_Fire"))
  (:`Triggered`
    (`|ExecutionSequence`
      (:`then_0`
        (`KismetSystemLibrary.Delay` 0.3)
        (if (`self.BP_Fire`)
          (`self.MouseLeft_FireTick` 0.0)))
      (:`then_1`
        (`self.CameraShakeTick` 0.0))))
  (:`Started`
    (`self.MouseLeft_FireStart`)
    (set `self.BP_Fire` true))
  (:`Completed`
    (`self.MouseLeft_FireEnd`)
    (set `self.BP_Fire` false)))

(event `EnhancedInput|/Game/Resources/TestLevel/Input/IA_G`
  (params (ActionValue :type Boolean) (ElapsedSeconds :type "Float (double-precision)") (TriggeredSeconds :type "Float (double-precision)") (InputAction :type "InputAction Object Reference" :default "/Game/Resources/TestLevel/Input/IA_G.IA_G"))
  ;[1 1 1] 아이템 떨어트리기
  (:`Triggered`
    (bind _asbp_character (cast `/Game/BluePrint/MainGameLevel/Character/BP_Character` (`GameplayStatics.GetPlayerCharacter` 0)))
    (`TestCharacter.DropItem` _asbp_character (`TestCharacter.CurItemIndex` _asbp_character))))

(event `EnhancedInput|/Game/Resources/TestLevel/Input/IA_Jump`
  (params (ActionValue :type Boolean) (ElapsedSeconds :type "Float (double-precision)") (TriggeredSeconds :type "Float (double-precision)") (InputAction :type "InputAction Object Reference" :default "/Game/Resources/TestLevel/Input/IA_Jump.IA_Jump"))
  (bind _returnvalue (`GameplayStatics.GetPlayerCharacter` 0))
  (:`Triggered`
    (`Character.Jump` _returnvalue))
  (:`Canceled`
    (`Character.StopJumping` _returnvalue :!label _label))
  (:`Completed`
    (goto _label)))

(event `EnhancedInput|/Game/Resources/TestLevel/Input/IA_AttackTest`
  (params (ActionValue :type Boolean) (ElapsedSeconds :type "Float (double-precision)") (TriggeredSeconds :type "Float (double-precision)") (InputAction :type "InputAction Object Reference" :default "/Game/Resources/TestLevel/Input/IA_AttackTest.IA_AttackTest")))

(event `EnhancedInput|/Game/Resources/TestLevel/Input/IA_Enter`
  (params (ActionValue :type Boolean) (ElapsedSeconds :type "Float (double-precision)") (TriggeredSeconds :type "Float (double-precision)") (InputAction :type "InputAction Object Reference" :default "/Game/Resources/TestLevel/Input/IA_Enter.IA_Enter"))
  (:`Triggered`
    (bind _asbp_main_title_hud (cast `/Game/BluePrint/MainGameLevel/UI/BP_MainTitleHUD` (`self.GetHUD`)))
    (`/Engine/EditorBlueprintResources/StandardMacros.IsValid` _asbp_main_title_hud
      (:`Is Valid`
        (`/Game/BluePrint/MainGameLevel/UI/BP_MainTitleHUD.EnterInput` _asbp_main_title_hud)))))

(event `EnhancedInput|/Game/Resources/TestLevel/Input/IA_Tab`
  (params (ActionValue :type Boolean) (ElapsedSeconds :type "Float (double-precision)") (TriggeredSeconds :type "Float (double-precision)") (InputAction :type "InputAction Object Reference" :default "/Game/Resources/TestLevel/Input/IA_Tab.IA_Tab")))

(event `EnhancedInput|/Game/Resources/TestLevel/Input/IA_Map`
  (params (ActionValue :type Boolean) (ElapsedSeconds :type "Float (double-precision)") (TriggeredSeconds :type "Float (double-precision)") (InputAction :type "InputAction Object Reference" :default "/Game/Resources/TestLevel/Input/IA_Map.IA_Map"))
  (:`Started`
    (bind _asbp_main_game_hud (cast `/Game/BluePrint/MainGameLevel/UI/BP_MainGameHUD` (`self.GetHUD`)))
    (`/Engine/EditorBlueprintResources/StandardMacros.IsValid` _asbp_main_game_hud
      (:`Is Valid`
        (`/Game/BluePrint/MainGameLevel/UI/BP_MainGameHUD.MapInput` _asbp_main_game_hud)))))

(event `self.ChangePostureToWidget`
  (params (_Posture :type "EPlayerUpperState Enum" :default "UArm_Idle"))
  (bind _asbp_main_game_hud (cast `/Game/BluePrint/MainGameLevel/UI/BP_MainGameHUD` (`self.GetHUD`)))
  (`/Engine/EditorBlueprintResources/StandardMacros.IsValid` _asbp_main_game_hud
    (:`Is Valid`
      (`/Game/BluePrint/MainGameLevel/UI/BP_MainGameHUD.Number_Key` _asbp_main_game_hud _Posture))))

(event `self.CallGetItemToWidget`
  (bind _asbp_main_game_hud (cast `/Game/BluePrint/MainGameLevel/UI/BP_MainGameHUD` (`self.GetHUD`)))
  (`/Engine/EditorBlueprintResources/StandardMacros.IsValid` _asbp_main_game_hud
    (:`Is Valid`
      (`/Game/BluePrint/MainGameLevel/UI/BP_MainGameHUD.CallGetItem` _asbp_main_game_hud))))

(event `self.BullitCountToHUD`
  (bind _asbp_main_game_hud (cast `/Game/BluePrint/MainGameLevel/UI/BP_MainGameHUD` (`self.GetHUD`)))
  (`/Engine/EditorBlueprintResources/StandardMacros.IsValid` _asbp_main_game_hud
    (:`Is Valid`
      (`/Game/BluePrint/MainGameLevel/UI/BP_MainGameHUD.MouseLeftCall` _asbp_main_game_hud))))

(fn `SetUpWeaponUI`
  (locals (NewLocalVar :type "WB_LeaderBoard Object Reference"))
  (if (`self.IsLocalController`)
    (bind _returnvalue (`|CreateWidget` "/Game/BluePrint/PartDevLevel/UI/LeaderBoard/WB_LeaderBoard.WB_LeaderBoard_C"))
    (bind _output_get (set `self.UI_Ref` _returnvalue))
    (`UserWidget.AddToViewport` _output_get 0)))

(fn `UserConstructionScript`)